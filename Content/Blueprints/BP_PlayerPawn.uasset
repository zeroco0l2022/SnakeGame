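; Player pawn Blueprint that puts a score widget on screen and keeps it updated as points are added.
; BeginPlay creates UI_Score and adds it to the viewport, and the AddPoints override calls the parent, then passes Points to the widget.
; The construction script adds a rotated child actor offset along X from PawnCamera, using the camera's world location as the relative transform.
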(event EventBeginPlay
  (bind _returnvalue (UserInterface|CreateWidget "/Game/Widgets/UI_Score.UI_Score_C"))
  (bind _output_get (Variables|Default|SetUI _returnvalue))
  (UserInterface|Viewport|AddtoViewport _output_get 0))

(event Collision|EventActorBeginOverlap
  (params (OtherActor :type Actor%20Object%20Reference)))

(event EventTick
  (params (DeltaSeconds :type Float%20%28single-precision%29)))

(event EventAddPoints
  (|CallParentFunction)
  (Default|UpdateScore (Variables|Default|GetUI) (Variables|Default|GetPoints)))

(fn ConstructionScript
  (bind _pawncamera (Variables|Default|GetPawnCamera))
  (bind _returnvalue (Transformation|GetWorldLocation _pawncamera))
  (AddComponent|AddChildActorComponent false (Math|Transform|MakeTransform (Math|Vector|MakeVector (+ (.x _returnvalue) 1e+03) (.y _returnvalue) (.z _returnvalue)) "90.000000,0.000000,0.000000" "1.000000,1.000000,1.000000")))